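; Boss enemy that patrols points, investigates noises and chases the player, showing a health widget and a win screen on defeat.
; PawnSensing drives AIMoveTo: sight starts a run to the player's last known position, then a look-around before resuming patrol.
; Stuns cost health and pause movement and sensing on a timer; re-stuns only reset it.
; Capsule hits damage the player or open doors, nudging the boss back.
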(event OnComponentHit(CapsuleComponent)
  (params (HitComponent :type Primitive%20Component%20Object%20Reference) (OtherActor :type Actor%20Object%20Reference) (OtherComp :type Primitive%20Component%20Object%20Reference) (NormalImpulse :type Vector :default "0, 0, 0") (Hit :type Hit%20Result%20Structure%20%28by%20ref%29))
  (bind _asbp_first_person_character (Utilities|Casting|CastToBP_FirstPersonCharacter OtherActor)
    (:then
      (Game|Damage|ApplyDamage _asbp_first_person_character 1e+01 0 0))
    (:CastFailed
      (bind _asbp_door (Utilities|Casting|CastToBP_Door OtherActor))
      (Default|OpenDoor _asbp_door)
      (if (Variables|Default|GetIsChasing)
        (Transformation|AddActorLocalOffset "-150.000000,0.000000,0.000000" true false)
        (else
          (Transformation|AddActorLocalOffset "-100.000000,0.000000,0.000000" true false))))))

(event Custom|GoToNextPatrolPoint
  (bind _mesh (Variables|Character|GetMesh))
  (if (not (Variables|Default|GetIsChasing))
    (if (> (Utilities|Array|Length (Variables|Default|GetPatrolPoints)) 0)
      (Variables|Default|SetEnemyState "NewEnumerator0")
      (Components|Animation|SetAnimation _mesh "/Game/CR/Demo/Animations/Manny/MM_Walk_Fwd.MM_Walk_Fwd")
      (Components|Animation|PlayAnimation _mesh "/Game/CR/Demo/Animations/Manny/MM_Walk_Fwd.MM_Walk_Fwd" true)
      (Variables|/Script/Engine.CharacterMovementComponent|SetMaxWalkSpeed (Variables|Character|GetCharacterMovement) (Variables|Default|GetWalkSpeed))
      (Variables|Default|SetCurrentPatrolIndex (Math|Integer|%(Integer) (+ (Variables|Default|GetCurrentPatrolIndex) 1) (Utilities|Array|Length (Variables|Default|GetPatrolPoints))))
      (AI|AIMoveTo self "0, 0, 0" (Utilities|Array|Get(acopy) (Variables|Default|GetPatrolPoints) (Variables|Default|GetCurrentPatrolIndex)) 5.0 false))))

(event Custom|OnSeePawn
  (params (Pawn :type Pawn%20Object%20Reference))
  (bind _asbp_first_person_character (Utilities|Casting|CastToBP_FirstPersonCharacter Pawn))
  (if (Variables|Default|GetIsChasing)
    _
    (else
      (Audio|PlaySoundatLocation "/Game/Assets/SFX/SFX_Enemy_See.SFX_Enemy_See" (Transformation|GetActorLocation self) "0, 0, 0" 1.0 1.0 0.0 0 0 0 0)))
  (CallFunction|StartChase _asbp_first_person_character))

(event Custom|StartChase
  (params (NewParam :type BP%20First%20Person%20Character%20Object%20Reference))
  (bind _mesh (Variables|Character|GetMesh))
  (Development|PrintString "Start Chase")
  (Variables|Default|SetEnemyState "NewEnumerator1")
  (Components|Animation|SetAnimation _mesh "/Game/CR/Demo/Animations/Manny/MM_Run_Fwd.MM_Run_Fwd")
  (Components|Animation|PlayAnimation _mesh "/Game/CR/Demo/Animations/Manny/MM_Run_Fwd.MM_Run_Fwd" true)
  (Variables|Default|SetIsChasing true)
  (Variables|/Script/Engine.CharacterMovementComponent|SetMaxWalkSpeed (Variables|Character|GetCharacterMovement) (Variables|Default|GetRunSpeed))
  (bind _output_get (Variables|Default|SetLastKnownPlayerLocation (Transformation|GetActorLocation NewParam)))
  (AI|AIMoveTo self _output_get 0 5.0 false
    (:OnSuccess
      (Transformation|AddActorLocalRotation "0.000000,90.000000,0.000000" false false)
      (Utilities|FlowControl|Delay 1.0)
      (Transformation|AddActorLocalRotation "0.000000,-180.000000,0.000000" false false)
      (Utilities|FlowControl|Delay 1.0)
      (Transformation|AddActorLocalRotation "0.000000,90.000000,0.000000" false false)
      (Variables|Default|SetIsChasing false)
      (CallFunction|GotoNextPatrolPoint))))

(event Custom|OnHearPawn
  (params (Instigator :type Pawn%20Object%20Reference) (Location :type Vector%20%28by%20ref%29) (Volume :type Float%20%28single-precision%29))
  (bind _mesh (Variables|Character|GetMesh))
  (if (not (Variables|Default|GetIsChasing))
    (Utilities|Casting|CastToBP_FirstPersonCharacter Instigator)
    (Variables|Default|SetEnemyState "NewEnumerator2")
    (Components|Animation|SetAnimation _mesh "/Game/CR/Demo/Animations/Manny/MM_Walk_Fwd.MM_Walk_Fwd")
    (Components|Animation|PlayAnimation _mesh "/Game/CR/Demo/Animations/Manny/MM_Walk_Fwd.MM_Walk_Fwd" true)
    (bind _output_get (Variables|Default|SetLastKnownPlayerLocation Location))
    (Variables|Default|SetIsSearching true)
    (AI|AIMoveTo self _output_get 0 5.0 false
      (:OnSuccess
        _)
      (:OnFail
        _))
    (Variables|Default|SetIsSearching false)
    (CallFunction|GotoNextPatrolPoint)))

(event Custom|ApplyStun
  (params (StunDuration :type Float%20%28double-precision%29))
  (bind _mesh (Variables|Character|GetMesh))
  (if (Variables|Default|GetIsStunned)
    (Utilities|Time|ClearTimerbyFunctionName 0 "EndStun")
    (Utilities|Time|SetTimerbyFunctionName 0 "EndStun" (Variables|Default|GetStunDuration))
    (else
      (bind _output_get (Variables|Default|SetHealth (- (Variables|Default|GetHealth) 10)))
      (Default|CallBHealthUpdate _output_get)
      (if (<= _output_get 0)
        (CallFunction|Defeat)
        (else
          (Variables|Default|SetIsStunned true)
          (Variables|Default|SetIsChasing false)
          (Variables|Default|SetPreStunSpeed (Variables|/Script/Engine.CharacterMovementComponent|GetMaxWalkSpeed (Variables|Character|GetCharacterMovement)))
          (Components|Animation|SetAnimation _mesh "/Game/CR/Demo/Animations/Manny/MM_Idle.MM_Idle")
          (Components|Animation|PlayAnimation _mesh "/Game/CR/Demo/Animations/Manny/MM_Idle.MM_Idle" true)
          (bind _asaicontroller (Utilities|Casting|CastToAIController (Pawn|GetController)))
          (AI|Navigation|StopMovement _asaicontroller)
          (Class|PawnSensingComponent|SetSensingUpdatesEnabled (Variables|Default|GetPawnSensing) false)
          (Utilities|Time|SetTimerbyFunctionName 0 "EndStun" (Variables|Default|GetStunDuration)))))))

(event Custom|EndStun
  (Variables|Default|SetIsStunned false)
  (Variables|/Script/Engine.CharacterMovementComponent|SetMaxWalkSpeed (Variables|Character|GetCharacterMovement) (Variables|Default|GetPreStunSpeed))
  (Class|PawnSensingComponent|SetSensingUpdatesEnabled (Variables|Default|GetPawnSensing) true)
  (CallFunction|GotoNextPatrolPoint))

(event Custom|OnActorHit_Event
  (params (SelfActor :type Actor%20Object%20Reference) (OtherActor :type Actor%20Object%20Reference) (NormalImpulse :type Vector) (Hit :type Hit%20Result%20Structure%20%28by%20ref%29))
  (EventDispatchers|BindEventtoOnActorHit (delegate Custom|OnActorHit_Event))
  (Development|PrintString "Hitting")
  (bind _asbp_first_person_character (Utilities|Casting|CastToBP_FirstPersonCharacter OtherActor)
    (:then
      (Game|Damage|ApplyDamage _asbp_first_person_character 1e+01 0 0))
    (:CastFailed
      (bind _asbp_door (Utilities|Casting|CastToBP_Door OtherActor))
      (Default|OpenDoor _asbp_door))))

(event EventBeginPlay
  (bind _mesh (Variables|Character|GetMesh))
  (bind _pawnsensing (Variables|Default|GetPawnSensing))
  (bind _returnvalue (UserInterface|CreateWidget "/Game/UI/BP_BossHealth.BP_BossHealth_C"))
  (Default|Initialize _returnvalue self)
  (UserInterface|Viewport|AddtoViewport _returnvalue 0)
  (EventDispatchers|BindEventtoOnSeePawn _pawnsensing (delegate Custom|OnSeePawn))
  (EventDispatchers|BindEventtoOnHearNoise _pawnsensing (delegate Custom|OnHearPawn))
  (Variables|/Script/Engine.CharacterMovementComponent|SetMaxWalkSpeed (Variables|Character|GetCharacterMovement) (Variables|Default|GetWalkSpeed))
  (if (> (Utilities|Array|Length (Variables|Default|GetPatrolPoints)) 0)
    (Components|Animation|SetAnimation _mesh "/Game/CR/Demo/Animations/Manny/MM_Walk_Fwd.MM_Walk_Fwd")
    (Components|Animation|PlayAnimation _mesh "/Game/CR/Demo/Animations/Manny/MM_Walk_Fwd.MM_Walk_Fwd" true)
    (AI|AIMoveTo self "0, 0, 0" (Utilities|Array|Get(acopy) (Variables|Default|GetPatrolPoints) (Variables|Default|GetCurrentPatrolIndex)) 5.0 false)))

(fn ConstructionScript)

(fn HitWallBounds
  (Development|PrintString "Stoping")
  (bind _asaicontroller (Utilities|Casting|CastToAIController (Pawn|GetController)))
  (AI|Navigation|StopMovement _asaicontroller)
  (Variables|Default|SetIsChasing false)
  (Variables|Default|SetIsSearching false)
  (Variables|Default|SetEnemyState "NewEnumerator0")
  (CallFunction|GotoNextPatrolPoint))

(fn Defeat
  (bind _returnvalue (Game|GetPlayerController 0))
  (Development|PrintString "defeat")
  (bind _returnvalue_2 (UserInterface|CreateWidget "/Game/UI/WBP_WinScreen.WBP_WinScreen_C"))
  (UserInterface|Viewport|AddtoViewport _returnvalue_2 0)
  (Input|SetInputModeUIOnly _returnvalue _returnvalue_2 "DoNotLock" false)
  (Variables|/Script/Engine.PlayerController|SetbShowMouseCursor _returnvalue true)
  (bind _outactors (Actor|GetAllActorsOfClass "/Game/Blueprints/BP_WeaponBase.BP_WeaponBase_C"))
  (Default|StopBlow _outactors)
  (Actor|DestroyActor))