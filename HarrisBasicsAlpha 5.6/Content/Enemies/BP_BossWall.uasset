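; Boss arena wall that seals behind the player and bounds the boss.
; When the player overlaps the Box trigger, it teleports them forward along their local X axis, makes the Cube solid and visible, and calls SpawnEnemy on the BP_BossSpawner actors.
; A boss overlapping the same trigger instead receives HitWallBounds.
; UndoWall hides the Cube and disables its collision to reopen the passage.
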(event OnComponentBeginOverlap(Box)
  (params (OverlappedComponent :type Primitive%20Component%20Object%20Reference) (OtherActor :type Actor%20Object%20Reference) (OtherComp :type Primitive%20Component%20Object%20Reference) (OtherBodyIndex :type Integer) (bFromSweep :type Boolean) (SweepResult :type Hit%20Result%20Structure%20%28by%20ref%29))
  (bind _asbp_boss (Utilities|Casting|CastToBP_Boss OtherActor)
    (:then
      (Default|HitWallBounds _asbp_boss))
    (:CastFailed
      (bind _asbp_first_person_character (Utilities|Casting|CastToBP_FirstPersonCharacter OtherActor))
      (Transformation|AddActorLocalOffset _asbp_first_person_character "100.000000,0.000000,0.000000" false true)
      (Collision|SetCollisionEnabled (Variables|Default|GetCube) "QueryAndPhysics")
      (Rendering|SetVisibility (Variables|Default|GetCube) true false)
      (Rendering|Material|SetMaterial (Variables|Default|GetCube) 0 "/Game/Textures/brick_Mat.brick_Mat")
      (bind _outactors (Actor|GetAllActorsOfClass "/Game/Enemies/BP_BossSpawner.BP_BossSpawner_C"))
      (Default|SpawnEnemy _outactors))))

(event EventBeginPlay)

(event Collision|EventActorBeginOverlap
  (params (OtherActor :type Actor%20Object%20Reference)))

(event EventTick
  (params (DeltaSeconds :type Float%20%28single-precision%29)))

(fn ConstructionScript)

(fn UndoWall
  (Collision|SetCollisionEnabled (Variables|Default|GetCube) "NoCollision")
  (Rendering|SetVisibility (Variables|Default|GetCube) false false)
  (Rendering|Material|SetMaterial (Variables|Default|GetCube) 0 "/Game/Textures/brick_Mat.brick_Mat"))