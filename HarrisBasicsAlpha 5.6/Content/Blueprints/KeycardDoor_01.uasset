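; KeycardDoor_01 is a hinged door that opens and closes on interaction when the player holds the white keycard.
; BeginPlay caches the player's BP_FirstPersonCharacter, and Interact checks its Keycards struct for that card.
; A FlipFlop alternately plays and reverses a Timeline that lerps the door's relative yaw to swing it open or shut.
; Interacting without the card does nothing.
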(event EventBeginPlay
  (bind _asbp_first_person_character (Utilities|Casting|CastToBP_FirstPersonCharacter (Game|GetPlayerCharacter 0)))
  (Variables|Default|SetAs%20BP%20First%20Person%20Character _asbp_first_person_character))

(event EventInteract
  (if (.Whitekeycard (Utilities|Struct|BreakKeycards (Variables|/Game/FirstPerson/Blueprints/BP_FirstPersonCharacter.BP_FirstPersonCharacter_C|GetKeycards (Variables|Default|GetAs%20BP%20First%20Person%20Character))))
    (Utilities|FlowControl|FlipFlop
      (:A
        (bind _newtrack_0 (Timeline|Timeline Play)
          (:Update
            (Transformation|SetRelativeRotation (Variables|Default|GetDoor) (Math|Rotator|MakeRotator 0.0 0.0 (Math|Float|Lerp 0.0 -1e+02 _newtrack_0)) false false))))
      (:B
        (Timeline|Timeline Reverse)))))

(fn ConstructionScript)