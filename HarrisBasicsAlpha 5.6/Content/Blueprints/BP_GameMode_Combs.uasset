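; Game mode that tracks a comb score and ends play with a win screen once the target count is reached.
; AddScore adds a delta to CurrentScore and calls ShowWinScreen when it meets or exceeds TargetCombs.
; ShowWinScreen adds the WBP_WinScreen widget to the viewport, switches input to UI only and pauses the game.
; The node that would show the mouse cursor is unconnected, so it never runs.
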(event Custom|AddScore
  (params (Delta :type Integer))
  (Variables|Default|SetCurrentScore (+ (Variables|Default|GetCurrentScore) Delta))
  (if (>= (Variables|Default|GetCurrentScore) (Variables|Default|GetTargetCombs))
    (CallFunction|ShowWinScreen)))

(event Custom|ShowWinScreen
  (bind _returnvalue (UserInterface|CreateWidget "/Game/UI/WBP_WinScreen.WBP_WinScreen_C"))
  (UserInterface|Viewport|AddtoViewport _returnvalue 0)
  (Input|SetInputModeUIOnly 0 0 "DoNotLock" false)
  (Game|SetGamePaused true))

(event EventBeginPlay)

(event EventTick
  (params (DeltaSeconds :type Float%20%28single-precision%29)))

(fn ConstructionScript)