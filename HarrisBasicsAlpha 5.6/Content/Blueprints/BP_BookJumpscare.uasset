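; BP_BookJumpscare is a one-time jumpscare that throws books when its trigger is overlapped.
; A DoOnce runs before the player check, so a non-player overlap first uses up the scare.
; For the player, it plays a chime at the actor's location, enables physics on a set of book components and pushes them along negative world X with a single AddForce call.
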(event OnComponentBeginOverlap(Trigger)
  (params (OverlappedComponent :type Primitive%20Component%20Object%20Reference) (OtherActor :type Actor%20Object%20Reference) (OtherComp :type Primitive%20Component%20Object%20Reference) (OtherBodyIndex :type Integer) (bFromSweep :type Boolean) (SweepResult :type Hit%20Result%20Structure%20%28by%20ref%29))
  (bind _book (Variables|Default|GetBook))
  (Utilities|FlowControl|DoOnce false
    (:Completed
      (if (== OtherActor (Game|GetPlayerCharacter 0))
        (Audio|PlaySoundatLocation "/Game/Assets/SFX/SFX_Chime_01A.SFX_Chime_01A" (Transformation|GetActorLocation) "0, 0, 0" 1.0 1.0 0.0 0 0 0 0)
        (Physics|SetSimulatePhysics _book true)
        (Physics|AddForce _book "-8000.000000,0.000000,0.000000" "None" false)))))

(fn ConstructionScript)