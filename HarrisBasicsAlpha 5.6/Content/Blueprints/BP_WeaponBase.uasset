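; BP_WeaponBase is a pickup blower weapon that stuns enemies in front of the player.
; Overlapping it fills and equips the character's slot 1, attaches it to the weapon anchor and enables the weapon input mapping.
; While slot 1 is active, shoot input toggles blow audio and FX, and sphere-traces along the camera rotation to stun BP_EnemyCharacter pawns.
; Tick stops the blow effects if another slot becomes active while blowing.
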(event OnComponentBeginOverlap(Collision)
  (params (OverlappedComponent :type Primitive%20Component%20Object%20Reference) (OtherActor :type Actor%20Object%20Reference) (OtherComp :type Primitive%20Component%20Object%20Reference) (OtherBodyIndex :type Integer) (bFromSweep :type Boolean) (SweepResult :type Hit%20Result%20Structure%20%28by%20ref%29))
  (bind _asbp_first_person_character (Utilities|Casting|CastToBP_FirstPersonCharacter OtherActor))
  (Variables|/Game/FirstPerson/Blueprints/BP_FirstPersonCharacter.BP_FirstPersonCharacter_C|SetWeaponSlot1 _asbp_first_person_character self)
  (Default|EquipSlot _asbp_first_person_character 1)
  (bind _output_get (Variables|Default|SetOwningCharacter _asbp_first_person_character))
  (Variables|/Game/FirstPerson/Blueprints/BP_FirstPersonCharacter.BP_FirstPersonCharacter_C|SetCurrentWeapon _asbp_first_person_character self)
  (Actor|SetOwner _asbp_first_person_character)
  (Transformation|AttachComponentToComponent (Variables|/Game/FirstPerson/Blueprints/BP_FirstPersonCharacter.BP_FirstPersonCharacter_C|GetWeaponAnchor _output_get) "" "SnapToTarget" "SnapToTarget" "SnapToTarget" true)
  (Variables|Default|SetIsEquipped true)
  (Collision|SetCollisionEnabled (Variables|Default|GetCollision) "NoCollision")
  (CallFunction|OnEquipped))

(event Custom|StartBlow
  (Audio|Components|Audio|Play (Variables|Default|GetBlowAudio) 0.0)
  (Components|Activation|Activate (Variables|Default|GetBlowFX) false))

(event Custom|StopBlow
  (Audio|Components|Audio|Stop (Variables|Default|GetBlowAudio))
  (Components|Activation|Deactivate (Variables|Default|GetBlowFX)))

(event Custom|OnEquipped
  (bind _returnvalue (Game|GetPlayerController 0))
  (Input|EnableInput _returnvalue)
  (Input|AddMappingContext (PlayerController|LocalPlayerSubsystems|GetEnhancedInputLocalPlayerSubsystem _returnvalue) "/Game/FirstPerson/Input/IMC_Weapons.IMC_Weapons" 0 "(bIgnoreAllPressedKeysUntilRelease=True,bForceImmediately=False,bNotifyUserSettings=False)"))

(event Input|EnhancedActionEvents|EnhancedInputActionIA_Shoot
  (params (ActionValue :type Boolean) (ElapsedSeconds :type Float%20%28double-precision%29) (TriggeredSeconds :type Float%20%28double-precision%29) (InputAction :type Input%20Action%20Object%20Reference :default "/Game/FirstPerson/Input/Actions/IA_Shoot.IA_Shoot"))
  (bind _returnvalue (Components|GetOwner))
  (bind _weaponmesh (Variables|Default|GetWeaponMesh))
  (bind _returnvalue_2 (Transformation|GetSocketLocation _weaponmesh "Center"))
  (:Triggered
    (bind _asbp_first_person_character (Utilities|Casting|CastToBP_FirstPersonCharacter _returnvalue))
    (if (== (Variables|/Game/FirstPerson/Blueprints/BP_FirstPersonCharacter.BP_FirstPersonCharacter_C|GetCurrentSlot _asbp_first_person_character) 1)
      (bind _outhits (Collision|MultiSphereTraceForObjects _returnvalue_2 (+ _returnvalue_2 (* (Math|Vector|RotateVector (Variables|Default|GetProjectileOffset) (Camera|GetCameraRotation (Game|GetPlayerCameraManager 0))) (Variables|Default|GetBlowRange))) 7e+01 (Utilities|Array|MakeArray "ObjectTypeQuery3") false 0 "None"))
      (for _array_element _outhits
        (bind _asbp_enemy_character (Utilities|Casting|CastToBP_EnemyCharacter (.HitActor (Collision|BreakHitResult _array_element))))
        (Default|ApplyStun _asbp_enemy_character 0.0))))
  (:Started
    (bind _asbp_first_person_character_2 (Utilities|Casting|CastToBP_FirstPersonCharacter _returnvalue))
    (if (== (Variables|/Game/FirstPerson/Blueprints/BP_FirstPersonCharacter.BP_FirstPersonCharacter_C|GetCurrentSlot _asbp_first_person_character_2) 1)
      (CallFunction|StartBlow)
      (Variables|Default|SetIsBlowing true)))
  (:Canceled
    (bind _asbp_first_person_character_3 (Utilities|Casting|CastToBP_FirstPersonCharacter (Components|GetOwner) :!label _label))
    (if (== (Variables|/Game/FirstPerson/Blueprints/BP_FirstPersonCharacter.BP_FirstPersonCharacter_C|GetCurrentSlot _asbp_first_person_character_3) 1)
      (CallFunction|StopBlow)
      (Variables|Default|SetIsBlowing false)))
  (:Completed
    (goto _label)))

(event EventTick
  (params (DeltaSeconds :type Float%20%28single-precision%29))
  (bind _asbp_first_person_character (Utilities|Casting|CastToBP_FirstPersonCharacter (Components|GetOwner)))
  (if (not (== (Variables|/Game/FirstPerson/Blueprints/BP_FirstPersonCharacter.BP_FirstPersonCharacter_C|GetCurrentSlot _asbp_first_person_character) 1))
    (if (Variables|Default|GetIsBlowing)
      (CallFunction|StopBlow))))

(fn ConstructionScript)